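; Wolf AI actor built on the Barghest skeletal mesh that wanders continuously through the level.
; A looping roam event moves it to random reachable points within a radius of its location, printing a message if a move fails.
; On BeginPlay it starts roaming, binds the tail and mane meshes to the body's pose via leader pose, and loops a walk animation as a test.
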(event `Random_Roam`
  (`|AIMoveTo` null (`NavigationSystemV1.K2_GetRandomReachablePointInRadius` (`self.K2_GetActorLocation`) 3000.0 null null) null
    (:`OnSuccess`
      (`self.Random_Roam`))
    (:`OnFail`
      (`KismetSystemLibrary.PrintString` "Unable to load"))))

(event `self.ReceiveBeginPlay`
  (`self.Random_Roam`)
  ;[1 1 1] Make the optional meshes to use the same skeleton as Barghest
  (`SkinnedMeshComponent.SetLeaderPoseComponent` (`self.SK_BARGHEST_TAIL`) (`self.SkeletalMeshComponent`) false false)
  (`SkinnedMeshComponent.SetLeaderPoseComponent` (`self.SK_BARGHEST_MANE`) (`self.SkeletalMeshComponent`) false false)
  ;[1 1 1] Perform a test animation in loop
  (`SkeletalMeshComponent.PlayAnimation` (`self.SkeletalMeshComponent`) "/Game/QuadrapedCreatures/Barghest/Animations/BARGHEST_walk.BARGHEST_walk" true))

(fn `UserConstructionScript`)