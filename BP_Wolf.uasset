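; BP_Wolf is a wolf AI pawn that roams at random and chases the player after sensing a pawn.
; From BeginPlay, a self-repeating event moves it to random reachable nearby points, with a delay between orders.
; PawnSensing sets IsSeenPlayer on any sighted pawn and triggers an AIMoveTo toward the first player character.
; The flag is never cleared, and the roam loop does not check it.
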(event `self.ReceiveBeginPlay`
  (`self.Roam_AI_Event`))

(event `Roam_AI_Event`
  (`|AIMoveTo` self (`NavigationSystemV1.K2_GetRandomReachablePointInRadius` (`self.K2_GetActorLocation`) 3000.0 null null) null 2000.0
    (:`then`
      (`KismetSystemLibrary.Delay` 2.0)
      (`self.Roam_AI_Event`))))

(event `self.PawnSensing.OnSeePawn`
  (params (Pawn :type "Pawn Object Reference"))
  (set `self.Is Seen Player` true)
  (`self.Follow_Player`))

(event `Follow_Player`
  (if (`self.Is Seen Player`)
    (`|AIMoveTo` self (0.0 0.0 0.0) (`GameplayStatics.GetPlayerCharacter` 0) 150.0)))

(fn `UserConstructionScript`)